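; Gameplay ability for a ranged attack that fires a projectile at the avatar's combat target.
; On activation it turns the avatar toward the target through interface messages and plays a random tagged attack montage.
; The montage's gameplay event tag times the projectile spawn, aimed at the target's current location.
; The ability ends shortly after firing, or when the montage completes, is interrupted or is cancelled.
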(event Ability|EventActivateAbility
  (bind _returnvalue (Ability|GetAvatarActorfromActorInfo))
  (bind _returnvalue_2 (Ability|GetAvatarActorfromActorInfo))
  (bind _returnvalue_3 (Class|EnemyInterface|GetCombatTarget(Message) _returnvalue_2))
  (Class|CombatInterface|UpdateFacingTarget(Message) _returnvalue_2 (Transformation|GetActorLocation _returnvalue_3))
  (bind _returnvalue_4 (Class|CombatInterface|GetAttackMontages(Message) (Ability|GetAvatarActorfromActorInfo)))
  (bind _output_get (Variables|Default|SetTaggedMontage (Class|AuraDamageGameplayAbility|GetRandomTaggedMontagefromArray _returnvalue_4)))
  (|PlayMontageandWaitProxy "None" (.Montage (Utilities|Struct|BreakTaggedMontage _output_get)) 1.0 "None" false 1.0 0.0 false
    (:then
      (Ability|Tasks|WaitGameplayEvent (.MontageTag (Utilities|Struct|BreakTaggedMontage _output_get)) 0
        (:EventReceived
          (Class|CombatInterface|GetCombatSocketLocation(Message) _returnvalue (.MontageTag (Utilities|Struct|BreakTaggedMontage _output_get)))
          (bind _returnvalue_5 (Class|EnemyInterface|GetCombatTarget(Message) _returnvalue))
          (Class|AuraProjectileSpell|SpawnProjectile (Transformation|GetActorLocation _returnvalue_5))
          (Utilities|FlowControl|Delay 0.5)
          (Ability|EndAbility))))
    (:OnCompleted
      (Ability|EndAbility :!label _label))
    (:OnInterrupted
      (goto _label))
    (:OnCancelled
      (goto _label))))

(event Ability|EventOnEndAbility
  (params (bWasCancelled :type Boolean)))